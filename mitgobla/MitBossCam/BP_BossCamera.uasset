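; BP_BossCamera is a camera actor that can orbit and watch a boss actor.
; BeginPlay applies configurable spotlight intensity and color, and copies post-process settings onto its scene capture component.
; Tick advances a slow, wrapping yaw angle, with separate toggles to aim the camera at BossRef and to place it on a raised circle around it.
; Aiming runs before the move, so it uses the pre-move location.
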(event `self.ReceiveBeginPlay`
  (bind _spotlight (`self.SpotLight`))
  (`LightComponent.SetIntensity` _spotlight (`self.LightIntensity`))
  (`LightComponent.SetLightColor` _spotlight (make `LinearColor` (`self.LightRed`) (`self.LightGreen`) (`self.LightBlue`) 1.0) true)
  (set `SceneCaptureComponent2D.PostProcessSettings` (`self.Post Process Settings`) (`self.SceneCaptureComponent2D`)))

(event `self.ReceiveTick`
  (params (DeltaSeconds :type "Float (single-precision)"))
  (bind _cameracomponent (`self.CameraComponent`))
  (bind _distancefromboss (`self.DistanceFromBoss`))
  (bind _returnvalue (`FSDConversionLibrary.ActorToWorldLocation` (`self.BossRef`)))
  (set `self.CurrentYawAngle` (+ (`self.CurrentYawAngle`) (* DeltaSeconds 5.0)))
  (if (> (`self.CurrentYawAngle`) 360.0)
    (set `self.CurrentYawAngle` 0.0))
  (if (`self.TrackBossRotation`)
    (`SceneComponent.K2_SetWorldRotation` _cameracomponent (`KismetMathLibrary.FindLookAtRotation` (`SceneComponent.K2_GetComponentLocation` _cameracomponent) _returnvalue) false false))
  (if (`self.TrackBossPosition`)
    (`SceneComponent.K2_SetWorldLocation` _cameracomponent (`KismetMathLibrary.MakeVector` (+ (.x _returnvalue) (* (`self.DistanceFromBoss`) (`KismetMathLibrary.DegSin` (`self.CurrentYawAngle`)))) (+ (.y _returnvalue) (* _distancefromboss (`KismetMathLibrary.DegCos` (`self.CurrentYawAngle`)))) (+ (.z _returnvalue) (* _distancefromboss 0.5))) false false)))

(fn `UserConstructionScript`)